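; Player controller for a networked ragdoll sync setup that shows the main widget for the local player and provides test hotkeys.
; F uses a FlipFlop to alternately start and stop ragdoll on every Ragdoll actor through its RagdollSyncComponent.
; R launches every physics-simulating Ragdoll mesh upward with a velocity-change impulse.
; Both keys act only with authority, so remote client presses do nothing.
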(event `self.ReceiveBeginPlay`
  (if (`self.IsLocalController`)
    (bind _returnvalue (`|CreateWidget` "/Game/UI/WBP_Main.WBP_Main_C" self))
    (`UserWidget.AddToViewport` _returnvalue 0)))

(event `Key|F`
  (params (Key :type "Key Structure"))
  (:`Pressed`
    (`/Engine/EditorBlueprintResources/ActorMacros.Switch Has Authority`
      (:`Authority`
        (bind _isa (`/Engine/EditorBlueprintResources/StandardMacros.FlipFlop`)
          (:`A`
            _)
          (:`B`
            _))
        (bind _outactors (`GameplayStatics.GetAllActorsOfClass` "/Script/RepRagdollSystem.Ragdoll"))
        (for _array_element _outactors
          (`/Engine/EditorBlueprintResources/StandardMacros.IsValid` _array_element
            (:`Is Valid`
              (bind _ragdollsynccomponent (`Ragdoll.RagdollSyncComponent` _array_element)
                (:`then`
                  (if _isa
                    (`RagdollSyncComponent.StartRagdoll` _ragdollsynccomponent)
                    (else
                      (`RagdollSyncComponent.StopRagdoll` _ragdollsynccomponent))))
                (:`else`)))))))))

(event `Key|R`
  (params (Key :type "Key Structure"))
  (:`Pressed`
    (`/Engine/EditorBlueprintResources/ActorMacros.Switch Has Authority`
      (:`Authority`
        (bind _outactors (`GameplayStatics.GetAllActorsOfClass` "/Script/RepRagdollSystem.Ragdoll"))
        (for _array_element _outactors
          (`/Engine/EditorBlueprintResources/StandardMacros.IsValid` _array_element
            (:`Is Valid`
              (bind _skeletalmeshcomponent (`Ragdoll.SkeletalMeshComponent` _array_element)
                (:`then`
                  (if (`SceneComponent.IsAnySimulatingPhysics` _skeletalmeshcomponent)
                    (`PrimitiveComponent.AddImpulse` _skeletalmeshcomponent (0.0 0.0 5000.0) "None" true)))
                (:`else`)))))))))

(fn `UserConstructionScript`)